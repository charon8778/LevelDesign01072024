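; Caged NPC actor in Level 1 that the player frees with a key, triggering its dialogue.
; A sphere overlap checks the first-person character's key flag; with a key, it destroys the cell mesh and moves the NPC to a hardcoded world position.
; After a short delay, a DoOnce starts the game mode's dialogue, disables character input and shows the cursor.
; Without a key, a flag-guarded no-key widget appears briefly.
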(event `self.Sphere.OnComponentBeginOverlap`
  (params (OverlappedComponent :type "PrimitiveComponent Object Reference") (OtherActor :type "Actor Object Reference") (OtherComp :type "PrimitiveComponent Object Reference") (OtherBodyIndex :type Integer) (bFromSweep :type Boolean) (SweepResult :type "HitResult Structure (by ref)"))
  (bind _asbp_first_person_character (cast `/Game/FirstPerson/Blueprints/BP_FirstPersonCharacter` OtherActor))
  (if (`/Game/FirstPerson/Blueprints/BP_FirstPersonCharacter.is Having Key?` _asbp_first_person_character)
    (`ActorComponent.K2_DestroyComponent` (`self.SM_cell_low`))
    (`SceneComponent.K2_SetWorldLocation` (`self.AI`) (-2580.0 790.0 720.0) false false)
    (`KismetSystemLibrary.Delay` 0.2)
    (bind _asbp_first_person_character_2 (cast `/Game/FirstPerson/Blueprints/BP_FirstPersonCharacter` OtherActor))
    (bind _asbp_first_person_game_mode (cast `/Game/FirstPerson/Blueprints/BP_FirstPersonGameMode` (`GameplayStatics.GetGameMode`)))
    (`/Engine/EditorBlueprintResources/StandardMacros.DoOnce` false
      (:`Completed`
        (`/Game/FirstPerson/Blueprints/BP_FirstPersonGameMode.StartDialogue` _asbp_first_person_game_mode "/Game/Level1/Dialogue/NPC2/NPCinCage.NPCinCage")
        (`self.DisableInput` _asbp_first_person_character_2 null)
        ;[1 1 1] cant see if checked context sensitive
        (set `PlayerController.bShowMouseCursor` true (`GameplayStatics.GetPlayerController` 0))))
    (else
      ;[0 0 0] widget show"no magic
      (if (not (`self.isWidgetVisible`))
        (bind _returnvalue (`|CreateWidget` "/Game/Level1/Dialogue/NPC2/W_noKey.W_noKey_C"))
        (`UserWidget.AddToViewport` _returnvalue 0)
        (set `self.isWidgetVisible` true)
        (`KismetSystemLibrary.Delay` 1.5)
        (`Widget.RemoveFromParent` _returnvalue)
        (set `self.isWidgetVisible` false)))))

(fn `UserConstructionScript`)