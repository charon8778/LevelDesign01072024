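; Quest-giver NPC Blueprint that starts a dialogue the first time the first-person character enters its trigger box.
; The overlap blends the view to the NPC, passes its Dialogue to the game mode, disables character input and shows the mouse cursor.
; After a short delay it reveals a tip TextRender.
; Turnofflight is an empty event, and the spawning and camera-return nodes are unconnected.
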(event `Turn off light`)

(event `self.ReceiveBeginPlay`)

(event `self.BoxTrigger.OnComponentBeginOverlap`
  (params (OverlappedComponent :type "PrimitiveComponent Object Reference") (OtherActor :type "Actor Object Reference") (OtherComp :type "PrimitiveComponent Object Reference") (OtherBodyIndex :type Integer) (bFromSweep :type Boolean) (SweepResult :type "HitResult Structure (by ref)"))
  (bind _asbp_first_person_character (cast `/Game/FirstPerson/Blueprints/BP_FirstPersonCharacter` OtherActor))
  (bind _asbp_first_person_game_mode (cast `/Game/FirstPerson/Blueprints/BP_FirstPersonGameMode` (`GameplayStatics.GetGameMode`)))
  (`/Engine/EditorBlueprintResources/StandardMacros.DoOnce` false
    (:`Completed`
      (`PlayerController.SetViewTargetWithBlend` (`GameplayStatics.GetPlayerController` 0) self 0.5 "VTBlend_Linear" 0.0 false)
      (`/Game/FirstPerson/Blueprints/BP_FirstPersonGameMode.StartDialogue` _asbp_first_person_game_mode (`self.Dialogue`))
      (`self.DisableInput` _asbp_first_person_character null)
      ;[1 1 1] cant see if checked context sensitive
      (set `PlayerController.bShowMouseCursor` true (`GameplayStatics.GetPlayerController` 0))
      (`KismetSystemLibrary.Delay` 0.1)
      ;[0 0 0] tips
      (`SceneComponent.SetVisibility` (`self.TextRender`) true false))))

(fn `UserConstructionScript`)