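; BP_FireProjectile is the fire attack projectile for Level1.
; Every tick it writes its world location into the MPC_fire material parameter collection, so materials can react to its position.
; On a box collision hit it calls the OnProjectileImpact dispatcher and spawns an explosion effect and sound at the impact point.
; It then destroys itself, after a short delay if the hit component uses MI_fire, otherwise immediately.
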(event `self.ReceiveTick`
  (params (DeltaSeconds :type "Float (single-precision)"))
  (`KismetMaterialLibrary.SetVectorParameterValue` "/Game/Level1/FireAttack/MPC_fire.MPC_fire" "Location" (`KismetMathLibrary.Conv_VectorToLinearColor` (`SceneComponent.K2_GetComponentLocation` (`self.Projectile`)))))

(event `self.BoxCollision.OnComponentHit`
  (params (HitComponent :type "PrimitiveComponent Object Reference") (OtherActor :type "Actor Object Reference") (OtherComp :type "PrimitiveComponent Object Reference") (NormalImpulse :type "Vector Structure") (Hit :type "HitResult Structure (by ref)"))
  (bind (_bblockinghit _binitialoverlap _time _distance _location) (`GameplayStatics.BreakHitResult` Hit))
  ;[0.3475 0.8184 1] Event Dispatches的自定义任务，右边添加input和input type
  (`self.OnProjectileImpact` OtherActor Hit)
  ;[0.9219 1 0.8438] sfx and vfx
  (`GameplayStatics.SpawnEmitterAtLocation` "/Game/01player/Ability/P_Gideon_Burden_HitWorld.P_Gideon_Burden_HitWorld" _location)
  (`GameplayStatics.PlaySoundAtLocation` "/Game/StarterContent/Audio/Explosion01.Explosion01" _location (struct) 1.0 1.0 0.0 null null null null)
  (if (== (`PrimitiveComponent.GetMaterial` OtherComp 0) "/Game/Level1/FireAttack/MI_fire.MI_fire")
    (`KismetSystemLibrary.PrintString` "equal")
    (`KismetSystemLibrary.Delay` 1.0)
    (`self.K2_DestroyActor`)
    (else
      (`KismetSystemLibrary.PrintString` "not equal")
      (`self.K2_DestroyActor`))))

(fn `UserConstructionScript`)