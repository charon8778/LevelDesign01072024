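; BPC_damageSystem is a Blueprint component that tracks health and death for the actor it is attached to.
; TakeDamage subtracts the incoming DamageInfo amount from CurrentHealth and sets IsDead once it reaches zero or below.
; It broadcasts OnDamageResponse with the damage response on surviving hits, and OnDeath on the fatal hit and any later hit.
; The function always returns true.
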(fn `Take damage`
  (params (DamageInfo :type "/Game/Level1/FireAttack/S_damageInfo Structure"))
  (returns (WasDamaged :type Boolean))
  (bind (_amount _damagetype _damageresponse) (break `/Game/Level1/FireAttack/S_damageInfo` DamageInfo))
  (if (not (`self.Is Dead`))
    (bind _output_get (set `self.CurrentHealth` (- (`self.CurrentHealth`) _amount)))
    ;[1 1 1] check if player is dead
    (if (<= _output_get 0.0)
      (set `self.Is Dead` true)
      (`self.OnDeath` :!label _label)
      (else
        (`self.OnDamageResponse` _damageresponse)))
    (else
      (goto _label)))
  (return true))